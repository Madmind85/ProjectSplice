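; Actor component that gives a character physical-animation hit reactions and ragdoll on its skeletal mesh, using a PhysicalAnimation component it adds at BeginPlay.
; HitReaction simulates bodies below the pelvis except the feet and applies an impulse along the hit trace, with strength chosen by whether the owner is dead.
; Tick fades the physics blend weight until simulation stops, or puts bodies to sleep after death.
; GoRagdoll switches to full simulation with the Ragdoll profile.
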(event Custom|TogglePhysicalAnimation
  (bind _physanimcomp (Variables|Default|GetPhysAnimComp))
  (Class|SkeletalMeshComponent|SetAllBodiesBelowSimulatePhysics (Variables|Default|GetMesh) (Utilities|Name|MakeLiteralName "pelvis") true false)
  (Class|PhysicalAnimationComponent|ApplyPhysicalAnimationProfileBelow _physanimcomp "pelvis" "None" false false)
  (Class|PhysicalAnimationComponent|SetStrengthMultiplyer _physanimcomp 2e+02)
  (Class|SkeletalMeshComponent|SetAllBodiesBelowPhysicsBlendWeight (Variables|Default|GetMesh) (Utilities|Name|MakeLiteralName "pelvis") 0.0 false true))

(event Custom|HitReaction
  (params (HitRes :type Hit%20Result%20Structure))
  (bind (_bblockinghit _binitialoverlap _time _distance _location _impactpoint _normal _impactnormal _physmat _hitactor _hitcomponent _hitbonename _bonename _hititem _elementindex _faceindex _tracestart _traceend) (Collision|BreakHitResult HitRes))
  (CallFunction|AdjustHitStrength)
  (Components|Tick|SetComponentTickEnabled true)
  (Variables|Default|SetHitReactionTimeRemaining (Variables|Default|GetHitReactionTime))
  (Class|PhysicalAnimationComponent|ApplyPhysicalAnimationProfileBelow (Variables|Default|GetPhysAnimComp) "pelvis" "Strong" false false)
  (Class|SkeletalMeshComponent|SetAllBodiesBelowSimulatePhysics (Variables|Default|GetMesh) (Utilities|Name|MakeLiteralName "pelvis") true false)
  (Class|SkeletalMeshComponent|SetAllBodiesBelowSimulatePhysics (Variables|Default|GetMesh) (Utilities|Name|MakeLiteralName "foot_r") false true)
  (Class|SkeletalMeshComponent|SetAllBodiesBelowSimulatePhysics (Variables|Default|GetMesh) (Utilities|Name|MakeLiteralName "foot_l") false true)
  (Physics|AddImpulse (Variables|Default|GetMesh) (* (Math|Vector|Normalize (- _traceend _tracestart)) (Variables|Default|GetHitStrength)) (select (== _hitbonename "pelvis") (Utilities|Name|MakeLiteralName "spine_01") _hitbonename) true))

(event EventBeginPlay
  (CallFunction|SetOwnerChar)
  (bind _returnvalue (Game|AddComponentbyClass (Components|GetOwner) "/Script/Engine.PhysicalAnimationComponent"))
  (bind _output_get (Variables|Default|SetPhysAnimComp _returnvalue))
  (bind _asmostriciattolo_5character (Utilities|Casting|CastToMostriciattolo5Character (Components|GetOwner)))
  (Variables|Default|SetMesh (Variables|/Script/Engine.Character|GetMesh _asmostriciattolo_5character))
  (Class|PhysicalAnimationComponent|SetSkeletalMeshComponent _output_get (Variables|/Script/Engine.Character|GetMesh _asmostriciattolo_5character)))

(event EventTick
  (params (DeltaSeconds :type Float%20%28single-precision%29))
  (if (Class|Mostriciattolo5Character|IsDead (Variables|Default|GetOwnerChar))
    (Utilities|FlowControl|Delay 2.0)
    (for _array_element (Transformation|GetAllSocketNames (Variables|Default|GetMesh))
      (Class|PrimitiveComponent|PutRigidBodytoSleep (Variables|Default|GetMesh) _array_element))
    (else
      (Variables|Default|SetHitReactionTimeRemaining (- (Math|Interpolation|FInterpTo (Variables|Default|GetHitReactionTimeRemaining) 0.0 0.0 0.1) (* DeltaSeconds 1.0)))
      (if (<= (Variables|Default|GetHitReactionTimeRemaining) 0.0)
        (Variables|Default|SetHitReactionTimeRemaining 0.0)
        (Class|SkeletalMeshComponent|SetAllBodiesBelowSimulatePhysics (Variables|Default|GetMesh) (Utilities|Name|MakeLiteralName "pelvis") false true)
        (Components|Tick|SetComponentTickEnabled false)
        (else
          (Class|SkeletalMeshComponent|SetAllBodiesBelowPhysicsBlendWeight (Variables|Default|GetMesh) (Utilities|Name|MakeLiteralName "pelvis") (Math|Float|Min(Float) (Variables|Default|GetHitReactionTimeRemaining) 1.0) false true))))))

(fn AdjustHitStrength
  (bind _returnvalue (Class|IntMCharacter|IntIsActorDead(Message) (Components|GetOwner)))
  (if _returnvalue
    (Variables|Default|SetHitStrength (Variables|Default|GetDeadHitStrength))
    (else
      (Variables|Default|SetHitStrength (Variables|Default|GetAliveHitStrength))))
  (return))

(fn SetOwnerChar
  (bind _asbp_third_person_character (Utilities|Casting|CastToBP_ThirdPersonCharacter (Components|GetOwner)))
  (Variables|Default|SetOwnerChar _asbp_third_person_character))

(fn GoRagdoll
  (Class|SkeletalMeshComponent|SetAllBodiesBelowSimulatePhysics (Variables|Default|GetMesh) (Utilities|Name|MakeLiteralName "pelvis") true true)
  (Components|Tick|SetComponentTickEnabled false)
  (Class|PhysicalAnimationComponent|ApplyPhysicalAnimationProfileBelow (Variables|Default|GetPhysAnimComp) "pelvis" "Ragdoll" true false)
  (Class|SkeletalMeshComponent|SetAllBodiesBelowSimulatePhysics (Variables|Default|GetMesh) (Utilities|Name|MakeLiteralName "pelvis") true true)
  (return))