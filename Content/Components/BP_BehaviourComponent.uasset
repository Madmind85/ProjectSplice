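; Actor component that manages an NPC's AI behaviour tree and blackboard for patrolling and reacting to a "Mostriciattolo" target.
; It starts the default tree on BeginPlay and feeds it patrol points from a looping Targets array.
; Helpers write spotted, status, aim and suspect-point keys, redirecting aim to the third-person character's TargetActor.
; Restart stops the tree, waits out a post-possession stun, then restarts it with cleared detection and reset walk speed.
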(event Custom|startBT
  (AI|RunBehaviorTree (AI|GetAIController (Components|GetOwner)) (Variables|Default|GetDefaultBehaviourTree))
  (CallFunction|SetNextTarget))

(event Custom|RestartBT
  (params (Owner :type Mostriciattolo%205%20Character%20Object%20Reference))
  (CallFunction|StopBT)
  (Utilities|FlowControl|Delay (Variables|Default|GetAfterPossessStunDuration))
  (CallFunction|StartBT)
  (CallFunction|SetMostriciattoloonBB 0 false)
  (Variables|/Script/Engine.CharacterMovementComponent|SetMaxWalkSpeed (Variables|/Script/Engine.Character|GetCharacterMovement Owner) 3e+02))

(event EventBeginPlay
  (CallFunction|StartBT))

(event EventTick
  (params (DeltaSeconds :type Float%20%28single-precision%29)))

(fn SetNextTarget
  (if (Utilities|IsValid (Utilities|Array|Get(acopy) (Variables|Default|GetTargets) (Variables|Default|GetCurrentTargetIndex)))
    (AI|Components|Blackboard|SetValueasVector (AI|GetBlackboard (Components|GetOwner)) (Variables|Default|GetNextTargetPoint) (Transformation|GetActorLocation (Utilities|Array|Get(acopy) (Variables|Default|GetTargets) (Variables|Default|GetCurrentTargetIndex))))
    (if (>= (Variables|Default|GetCurrentTargetIndex) (- (Utilities|Array|Length (Variables|Default|GetTargets)) 1))
      (Variables|Default|SetCurrentTargetIndex 0)
      (else
        (Math|Integer|IncrementInt (Variables|Default|GetCurrentTargetIndex)
          (:%20%20
            _))))
    (return)))

(fn SetMostriciattoloonBB
  (params (Mostriciattolo :type Actor%20Object%20Reference) (MostriciattoloSpotted :type Boolean) (CurrentStatus :type Byte))
  (AI|Components|Blackboard|SetValueasObject (AI|GetBlackboard (Components|GetOwner)) (Variables|Default|GetMostriciattolo) Mostriciattolo)
  (AI|Components|Blackboard|SetValueasBool (AI|GetBlackboard (Components|GetOwner)) (Variables|Default|GetMostriciattoloSpotted) MostriciattoloSpotted)
  (AI|Components|Blackboard|SetValueasEnum (AI|GetBlackboard (Components|GetOwner)) (Variables|Default|GetCurrentStatus) CurrentStatus)
  (bind _asbp_third_person_character (Utilities|Casting|CastToBP_ThirdPersonCharacter Mostriciattolo)
    (:then
      (AI|Components|Blackboard|SetValueasObject (AI|GetBlackboard (Components|GetOwner)) (Variables|Default|GetAimTarget) (Variables|/Game/Characters/Enemies/BP_ThirdPersonCharacter.BP_ThirdPersonCharacter_C|GetTargetActor _asbp_third_person_character)))
    (:CastFailed
      (AI|Components|Blackboard|SetValueasObject (AI|GetBlackboard (Components|GetOwner)) (Variables|Default|GetAimTarget) Mostriciattolo)))
  (return))

(fn SetMostriciattoloSpotted
  (params (BoolValue :type Boolean))
  (AI|Components|Blackboard|SetValueasBool (AI|GetBlackboard (Components|GetOwner)) (Variables|Default|GetMostriciattoloSpotted) BoolValue)
  (return))

(fn SetNPCtoAttento
  (params (Target :type Mostriciattolo%205%20Character%20Object%20Reference) (CurrentStatus :type Byte))
  (bind _returnvalue (Components|GetOwner))
  (bind _returnvalue_2 (AI|GetBlackboard _returnvalue))
  (AI|Components|Blackboard|SetValueasObject _returnvalue_2 (Variables|Default|GetMostriciattolo) Target)
  (if (== (Class|BlackboardComponent|GetValueasEnum _returnvalue_2 (Variables|Default|GetCurrentStatus)) 2)
    _
    (else
      (AI|Components|Blackboard|SetValueasVector (AI|GetBlackboard (Components|GetOwner)) (Variables|Default|GetSuspectPoint) (Transformation|GetActorLocation Target))
      (AI|Components|Blackboard|SetValueasEnum (AI|GetBlackboard (Components|GetOwner)) (Variables|Default|GetCurrentStatus) CurrentStatus)))
  (return))

(fn StopBT
  (CallFunction|SetMostriciattoloonBB 0 false)
  (AI|Logic|StopLogic (Variables|/Script/AIModule.AIController|GetBrainComponent (AI|GetAIController (Components|GetOwner))) "DEAD")
  (return))