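; BP_Rifle is a rifle pickup and weapon that supplies firing and melee feedback for the character holding it.
; Box overlap toggles the interact prompt on BPI_Character actors, and Interact hands the rifle to Mostriciattolo5Character via SetWeapon.
; ShootEffect plays sound, emits AI-audible "Pericolo" noise only for possessed shooters, and adds camera shake and recoil for the player.
; Animations route to the owner through interface messages, including Explode, which destroys the rifle.
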(event OnComponentBeginOverlap(Box)
  (params (OverlappedComponent :type Primitive%20Component%20Object%20Reference) (OtherActor :type Actor%20Object%20Reference) (OtherComp :type Primitive%20Component%20Object%20Reference) (OtherBodyIndex :type Integer) (bFromSweep :type Boolean) (SweepResult :type Hit%20Result%20Structure%20%28by%20ref%29))
  (if (not (Variables|Default|GetBeingHeld))
    (if (Utilities|DoesObjectImplementInterface OtherActor "/Game/BP_Interfaces/BPI_Character.BPI_Character_C")
      (Class|BPICharacter|InteractWidget(Message) OtherActor self true (Variables|Default|GetInteractableActorName)))))

(event OnComponentEndOverlap(Box)
  (params (OverlappedComponent :type Primitive%20Component%20Object%20Reference) (OtherActor :type Actor%20Object%20Reference) (OtherComp :type Primitive%20Component%20Object%20Reference) (OtherBodyIndex :type Integer))
  (if (Utilities|DoesObjectImplementInterface OtherActor "/Game/BP_Interfaces/BPI_Character.BPI_Character_C")
    (Class|BPICharacter|InteractWidget(Message) OtherActor self false "")))

(event Custom|WeaponBash_1
  (Class|BPICharacter|IntPlayAnimMont(Message) (Components|GetOwner) "/Game/Characters/Enemies/Animations/ANIM_NPC_Melee_Montage.ANIM_NPC_Melee_Montage"))

(event EventBeginPlay)

(event EventTick
  (params (DeltaSeconds :type Float%20%28single-precision%29)))

(event EventWeaponEffect
  (bind _returnvalue (Components|GetOwner))
  (Audio|PlaySoundatLocation "/Game/Effects/Sounds/NPC/punch-03_Cue.punch-03_Cue" (Transformation|GetActorLocation) "0, 0, 0" 1.0 1.0 0.0 0 0 0 0)
  (if (== _returnvalue (Pawn|GetControlledPawn (Game|GetPlayerController 0)))
    (Class|BpInterfaceCharacter|CameraShake(Message) _returnvalue "Shoot1")))

(event EventWeaponAnim
  (bind _returnvalue (Components|GetOwner))
  (if (Utilities|DoesObjectImplementInterface _returnvalue "/Game/BP_Interfaces/BPI_Character.BPI_Character_C")
    (Class|BPICharacter|IntPlayAnimMont(Message) _returnvalue (Variables|Default|GetAnim%20Mont))))

(event EventShootEffect
  (CallFunction|ShootEffect))

(event EventInteract
  (params (PlayerCharacter :type Character%20Object%20Reference))
  (bind _asmostriciattolo_5character (Utilities|Casting|CastToMostriciattolo5Character PlayerCharacter))
  (Class|Mostriciattolo5Character|SetWeapon _asmostriciattolo_5character self))

(fn ConstructionScript)

(fn ShootEffect
  (bind _returnvalue (Components|GetOwner))
  (bind _returnvalue_2 (Components|GetOwner))
  (Audio|PlaySoundatLocation (Variables|Default|GetWeaponAttackSound) (Transformation|GetActorLocation) "0, 0, 0" 1.0 1.0 0.0 0 0 0 0)
  ;[1 1 1] ai sente il suono solo se chi spara è posseduto
  (bind _asmostriciattolo_5character (Utilities|Casting|CastToMostriciattolo5Character _returnvalue_2))
  (if (Variables|/Script/Mostriciattolo5.Mostriciattolo5Character|GetIsBeingPossessed _asmostriciattolo_5character)
    (Class|Actor|MakeNoise self 8.0 _asmostriciattolo_5character (Transformation|GetActorLocation _returnvalue_2) 2e+02 "Pericolo"))
  (if (== _returnvalue (Pawn|GetControlledPawn (Game|GetPlayerController 0)))
    ;[1 1 1] ontroller
    (Class|BpInterfaceCharacter|CameraShake(Message) _returnvalue (Variables|Default|GetCameraShakeName))
    ;[1 1 1] recoil
    (Class|PlayerController|AddPitchInput (Game|GetPlayerController (Game|GetPlayerState 0)) (Variables|Default|GetRecoilAmount))))

(fn Explode
  (Effects|SpawnEmitterAttached "/Game/Effects/P_ky_explosion.P_ky_explosion" (Variables|Default|GetRoot) "None")
  (Class|BPICharacter|IntPlayAnimMont(Message) (Components|GetOwner) "/Game/Characters/Enemies/Animations/ANIM_NPC_WeaponExplode_Montage.ANIM_NPC_WeaponExplode_Montage")
  (Actor|DestroyActor))