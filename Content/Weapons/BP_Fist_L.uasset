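; BP_Fist_L is a fist weapon, likely the left hand, that supplies punch feedback and combo animations.
; WeaponEffect plays a punch sound at the fist and sends a camera shake message to the owner only when it is the first player's controlled pawn.
; WeaponAnim checks that the owner implements BPI_Character, then messages it to play one of three montages chosen by ComboIndex.
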(event EventBeginPlay)

(event Collision|EventActorBeginOverlap
  (params (OtherActor :type Actor%20Object%20Reference)))

(event EventTick
  (params (DeltaSeconds :type Float%20%28single-precision%29)))

(event EventWeaponEffect
  (bind _returnvalue (Components|GetOwner))
  (Audio|PlaySoundatLocation "/Game/Effects/Sounds/NPC/punch-03_Cue.punch-03_Cue" (Transformation|GetActorLocation) "0, 0, 0" 1.0 1.0 0.0 0 0 0 0)
  (if (== _returnvalue (Pawn|GetControlledPawn (Game|GetPlayerController 0)))
    (Class|BpInterfaceCharacter|CameraShake(Message) _returnvalue "Shoot1")))

(event EventWeaponAnim
  (bind _returnvalue (Components|GetOwner))
  (if (Utilities|DoesObjectImplementInterface _returnvalue "/Game/BP_Interfaces/BPI_Character.BPI_Character_C")
    (switch int (Variables|Default|GetComboIndex)
      (:Default
        (Class|BPICharacter|IntPlayAnimMont(Message) _returnvalue (Variables|Default|GetAnimMont_2)))
      (:0
        (Class|BPICharacter|IntPlayAnimMont(Message) _returnvalue (Variables|Default|GetAnimMont_0)))
      (:1
        (Class|BPICharacter|IntPlayAnimMont(Message) _returnvalue (Variables|Default|GetAnimMont_1))))))

(fn ConstructionScript)