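; BP_Mostriciattolo is the player creature character that possesses NPCs and can return to its own body.
; Input drives movement, camera lean, target cycling, focus mode and possession, with parent-class functions handling much of the logic.
; Possession and depossession combine motion-warped montages, level sequences and camera re-attachment.
; Frontal possession adds a timed key-mashing QTE, whose TapKey UI result selects the win or lose sequence.
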(event Custom|Create%20Tap%20Key%20Event
  (params (Tanget%20Key :type Key%20Structure :default "None") (Target%20Key%20%28as%20text%29 :type Text) (Timed? :type Boolean) (Duration :type Float%20%28double-precision%29) (Called%20from :type Actor%20Object%20Reference))
  ;[0.1939 0.6609 1] QuickTimeEvent
  (Variables|Default|SetTap%20Key%20Actor%20reference Called%20from)
  (bind _returnvalue (UserInterface|CreateWidget "/Game/Sequencer/TapKeySystem/Widget/TapKey_UI.TapKey_UI_C"))
  (UserInterface|Viewport|AddtoViewport _returnvalue 0)
  (Class|UserWidget|SetPositioninViewport _returnvalue "(X=550.000000,Y=500.000000)" true) ; Per ora è 2d, vediamo se riusciremo a farlo in 3d
  (Variables|Default|SetCurrent%20Tap%20Key%20reference _returnvalue)
  (Variables|/Game/Sequencer/TapKeySystem/Widget/TapKey_UI.TapKey_UI_C|SetKey (Variables|Default|GetCurrent%20Tap%20Key%20reference) Tanget%20Key)
  (Variables|Default|SetIn%20Tap%20Key%20progress? true)
  (Default|SetText (Variables|Default|GetCurrent%20Tap%20Key%20reference) Target%20Key%20%28as%20text%29)
  (if Timed?
    (Components|Timeline|SetPlayRate (Variables|Default|GetDuration%20progress%20Timeline) (/ 1.0 Duration))
    (bind _value (Timeline|Duration%20progress%20Timeline PlayFromStart)
      (:Update
        (Progress|SetPercent (Variables|/Game/Sequencer/TapKeySystem/Widget/TapKey_UI.TapKey_UI_C|GetTimerBar (Variables|Default|GetCurrent%20Tap%20Key%20reference)) (Math|Float|Lerp 1.0 0.0 _value)))
      (:Finished
        (if (Variables|Default|GetIn%20Tap%20Key%20progress?)
          (UserInterface|Animation|PlayAnimation (Variables|Default|GetCurrent%20Tap%20Key%20reference) (Variables|/Game/Sequencer/TapKeySystem/Widget/TapKey_UI.TapKey_UI_C|GetFailed (Variables|Default|GetCurrent%20Tap%20Key%20reference)) 0.0 1 "Forward" 1.0 false)
          (Class|TapKeyInterface|TapKeyFailedScript(Message) (Variables|Default|GetTap%20Key%20Actor%20reference)))
        (Variables|/Game/Sequencer/TapKeySystem/Widget/TapKey_UI.TapKey_UI_C|SetTap%20Key%20Progress (Variables|Default|GetCurrent%20Tap%20Key%20reference) 0.0)
        (Variables|Default|SetIn%20Tap%20Key%20progress? false)))))

(event EventInteractWidget
  (params (InteractableActor :type Actor%20Object%20Reference) (IsInRange :type Boolean) (ActorName :type Name :default "None"))
  (bind _currentinteractablewidget (Variables|Default|GetCurrentInteractableWidget))
  (bind _currentinteractablewidget_2 (Variables|Default|GetCurrentInteractableWidget))
  (if IsInRange
    (Variables|/Game/UserInterface/BPW_InteractableText.BPW_InteractableText_C|SetLookedAtObject _currentinteractablewidget_2 InteractableActor)
    (Variables|/Game/UserInterface/BPW_InteractableText.BPW_InteractableText_C|SetActorName _currentinteractablewidget_2 (Utilities|Text|ToText(Name) ActorName))
    (else
      (Variables|/Game/UserInterface/BPW_InteractableText.BPW_InteractableText_C|SetLookedAtObject _currentinteractablewidget 0)
      (Variables|/Game/UserInterface/BPW_InteractableText.BPW_InteractableText_C|SetActorName _currentinteractablewidget ""))))

(event Collision|EventActorBeginOverlap
  (params (OtherActor :type Actor%20Object%20Reference)))

(event EventBeginPlay
  ;[0.2083 0.07315 0.05027] BeginPlay
  ;;[1 1 1] BeginPlay
  (CallFunction|LeanCameraE)
  ;;[1 1 1] blocca l'altezza massima di visuale per non dare problemi
  (Variables|/Script/Engine.PlayerCameraManager|SetViewPitchMax (Variables|/Script/Engine.PlayerController|GetPlayerCameraManager (Game|GetPlayerController 0)) 5.0)
  (Utilities|IsValid (Variables|Default|GetCurrentInteractableWidget)
    (:Is%20Not%20Valid
      (bind _returnvalue (UserInterface|CreateWidget "/Game/UserInterface/BPW_InteractableText.BPW_InteractableText_C"))
      (bind _output_get (Variables|Default|SetCurrentInteractableWidget _returnvalue))
      (UserInterface|Viewport|AddtoViewport _output_get 0)
      (bind _asbp_mostriciattolo_game_mode (Utilities|Casting|CastToBP_MostriciattoloGameMode (Game|GetGameMode)))
      (Utilities|FlowControl|Delay 0.2)
      (Variables|/Script/Mostriciattolo5.Mostriciattolo5GameMode|SetMostriciattolo_OS _asbp_mostriciattolo_game_mode self))))

(event EventTick
  (params (DeltaSeconds :type Float%20%28single-precision%29)))

(event Input|KeyboardEvents|AnyKey
  (params (Key :type Key%20Structure))
  (bind _current_tap_key_reference (Variables|Default|GetCurrent%20Tap%20Key%20reference))
  ;[0.1939 0.6609 1] QuickTimeEvent
  ;;[0.7057 1 0.6784] Listen for any key being pressed, and if a tap key event is in progress, check if the correct key is being pressed, if yes then add a float to the progress on each press. if max reached then play SUCCESS Animation
  (:Pressed
    (if (Variables|Default|GetIn%20Tap%20Key%20progress?)
      (if (== Key (Variables|/Game/Sequencer/TapKeySystem/Widget/TapKey_UI.TapKey_UI_C|GetKey (Variables|Default|GetCurrent%20Tap%20Key%20reference)))
        (bind _output_get (Variables|/Game/Sequencer/TapKeySystem/Widget/TapKey_UI.TapKey_UI_C|SetTap%20Key%20Progress (Variables|Default|GetCurrent%20Tap%20Key%20reference) (Math|Float|Clamp(Float) (+ (Variables|/Game/Sequencer/TapKeySystem/Widget/TapKey_UI.TapKey_UI_C|GetTap%20Key%20Progress (Variables|Default|GetCurrent%20Tap%20Key%20reference)) 0.05))))
        (if (and (>= _output_get 1.0) (Variables|Default|GetIn%20Tap%20Key%20progress?))
          (UserInterface|Animation|PlayAnimation _current_tap_key_reference (Variables|/Game/Sequencer/TapKeySystem/Widget/TapKey_UI.TapKey_UI_C|GetPassed _current_tap_key_reference) 0.0 1 "Forward" 1.0 false)
          (Class|TapKeyInterface|TapKeyPassedScript(Message) (Variables|Default|GetTap%20Key%20Actor%20reference))
          (Variables|Default|SetIn%20Tap%20Key%20progress? false))))))

(fn ConstructionScript
  (bind _returnvalue (Rendering|Material|CreateDynamicMaterialInstance (Variables|Character|GetMesh) 0 "/Game/Characters/Creature/Materials/MI_Creature.MI_Creature" "None" :!class /Script/Engine.PrimitiveComponent))
  (Variables|MaterialParameters|SetMI_Creature _returnvalue))

(fn SwapActor
  (params (InPawn :type Pawn%20Object%20Reference))
  (Collision|SetCollisionEnabled (Variables|Character|GetMesh) "NoCollision")
  (Collision|SetCollisionEnabled (Variables|Default|GetCapsuleComponent) "NoCollision")
  (Pawn|Possess (Game|GetPlayerController (Variables|/Script/Engine.Pawn|GetPlayerState (Game|Player|GetPlayerPawn 0))) InPawn))

(fn SetCameraYLocation
  (params (New%20Location%20Y :type Float%20%28double-precision%29))
  (Variables|/Script/Engine.SpringArmComponent|SetSocketOffset (Variables|Default|GetSpringArm) (Math|Vector|MakeVector 0.0 New%20Location%20Y 0.0)))

(fn PlayCameraShakebyName
  (params (NewParam :type Name))
  (bind _asbp_mostriciattolo_game_mode (Utilities|Casting|CastToBP_MostriciattoloGameMode (Game|GetGameMode)))
  (Default|PlayShakebyName _asbp_mostriciattolo_game_mode NewParam))

(fn PlayWalkShake
  (CallFunction|PlayCameraShakebyName "Walk"))

(fn BPIGetHasWeapon
  (return false 0))

(fn BPIGetPatrolRoute
  (return 0))

(fn BPIGetRandomPointforShooting
  (params (Target%20Actor :type Actor%20Object%20Reference))
  (return "0, 0, 0"))

(fn BPIStartVault
  (return false))

(event Custom|LeanCameraE
  ;[1 1 1] Camera Move OverTime
  (Utilities|FlowControl|FlipFlop
    (:A
      (Class|ValueOverTimeComponent|StartCameraMoveOverTime (Variables|Default|GetBP_ValueOverTimeComponent) true))
    (:B
      (Class|ValueOverTimeComponent|StartCameraMoveOverTime (Variables|Default|GetBP_ValueOverTimeComponent) false))))

(event Input|EnhancedActionEvents|EnhancedInputActionCrouch
  (params (ActionValue :type Boolean) (ElapsedSeconds :type Float%20%28double-precision%29) (TriggeredSeconds :type Float%20%28double-precision%29) (InputAction :type Input%20Action%20Object%20Reference :default "/Game/Characters/Creature/Input/Actions/Crouch.Crouch"))
  ;[1 1 1] Crouch
  (:Triggered
    (Utilities|FlowControl|FlipFlop
      (:A
        (Character|Crouch))
      (:B
        (Character|UnCrouch)))))

(event Input|EnhancedActionEvents|EnhancedInputActionToggleSelectMode
  (params (ActionValue :type Boolean) (ElapsedSeconds :type Float%20%28double-precision%29) (TriggeredSeconds :type Float%20%28double-precision%29) (InputAction :type Input%20Action%20Object%20Reference :default "/Game/Characters/Creature/Input/Actions/ToggleSelectMode.ToggleSelectMode"))
  ;[1 1 1] ToggleSelectMode
  (:Triggered
    (bind _returnvalue (Class|Mostriciattolo5Character|StartSelectFocusMode))
    (if (not _returnvalue)
      (Variables|/Script/CinematicCamera.CineCameraComponent|SetFocusSettings (Variables|Default|GetCineCameraCreature) (Utilities|Struct|MakeCameraFocusSettings "Manual" 1e+02 "(ActorToTrack=None,RelativeOffset=(X=0.000000,Y=0.000000,Z=0.000000))" false 8.0 0.0)))))

(event Input|EnhancedActionEvents|EnhancedInputActionIA_JogOverride
  (params (ActionValue :type Boolean) (ElapsedSeconds :type Float%20%28double-precision%29) (TriggeredSeconds :type Float%20%28double-precision%29) (InputAction :type Input%20Action%20Object%20Reference :default "/Game/Characters/Creature/Input/Actions/IA_JogOverride.IA_JogOverride"))
  ;[1 1 1] JobOverride
  (:Triggered
    (Variables|/Script/Engine.CharacterMovementComponent|SetMaxWalkSpeed (Variables|Character|GetCharacterMovement) 5e+02))
  (:Canceled
    (Variables|/Script/Engine.CharacterMovementComponent|SetMaxWalkSpeed (Variables|Character|GetCharacterMovement) 1e+02 :!label _label))
  (:Completed
    (goto _label)))

(event Input|EnhancedActionEvents|EnhancedInputActionIA_LookUP
  (params (ActionValue :type Float%20%28double-precision%29) (ElapsedSeconds :type Float%20%28double-precision%29) (TriggeredSeconds :type Float%20%28double-precision%29) (InputAction :type Input%20Action%20Object%20Reference :default "/Game/Characters/Creature/Input/Actions/IA_LookUP.IA_LookUP"))
  ;[1 1 1] Look
  (:Triggered
    (Class|Mostriciattolo5Character|Look (Utilities|Struct|MakeInputActionValue 0.0 ActionValue 0.0 "Axis2D"))))

(event Input|EnhancedActionEvents|EnhancedInputActionIA_LookTurn
  (params (ActionValue :type Float%20%28double-precision%29) (ElapsedSeconds :type Float%20%28double-precision%29) (TriggeredSeconds :type Float%20%28double-precision%29) (InputAction :type Input%20Action%20Object%20Reference :default "/Game/Characters/Creature/Input/Actions/IA_LookTurn.IA_LookTurn"))
  ;[1 1 1] Look
  (:Triggered
    (Class|Mostriciattolo5Character|Look (Utilities|Struct|MakeInputActionValue ActionValue 0.0 0.0 "Axis2D"))))

(event Input|EnhancedActionEvents|EnhancedInputActionIA_Move_Forward
  (params (ActionValue :type Float%20%28double-precision%29) (ElapsedSeconds :type Float%20%28double-precision%29) (TriggeredSeconds :type Float%20%28double-precision%29) (InputAction :type Input%20Action%20Object%20Reference :default "/Game/Characters/Creature/Input/Actions/IA_Move_Forward.IA_Move_Forward"))
  ;[1 1 1] Move
  (:Triggered
    (Class|Mostriciattolo5Character|Move (Utilities|Struct|MakeInputActionValue 0.0 ActionValue 0.0 "Axis3D"))))

(event Input|EnhancedActionEvents|EnhancedInputActionIA_Move_Right
  (params (ActionValue :type Float%20%28double-precision%29) (ElapsedSeconds :type Float%20%28double-precision%29) (TriggeredSeconds :type Float%20%28double-precision%29) (InputAction :type Input%20Action%20Object%20Reference :default "/Game/Characters/Creature/Input/Actions/IA_Move_Right.IA_Move_Right"))
  ;[1 1 1] Move
  (:Triggered
    (Class|Mostriciattolo5Character|Move (Utilities|Struct|MakeInputActionValue ActionValue 0.0 0.0 "Axis3D"))))

(event Input|EnhancedActionEvents|EnhancedInputActionCameraLean
  (params (ActionValue :type Boolean) (ElapsedSeconds :type Float%20%28double-precision%29) (TriggeredSeconds :type Float%20%28double-precision%29) (InputAction :type Input%20Action%20Object%20Reference :default "/Game/Characters/Creature/Input/Actions/CameraLean.CameraLean"))
  ;[1 1 1] CameraLean
  (:Triggered
    (CallFunction|LeanCameraE)))

(event Input|EnhancedActionEvents|EnhancedInputActionPossess
  (params (ActionValue :type Boolean) (ElapsedSeconds :type Float%20%28double-precision%29) (TriggeredSeconds :type Float%20%28double-precision%29) (InputAction :type Input%20Action%20Object%20Reference :default "/Game/Characters/Creature/Input/Actions/Possess.Possess"))
  ;[1 1 1] Possess
  (:Ongoing
    (Class|Mostriciattolo5Player|InterceptPossessPoint)))

(event Input|EnhancedActionEvents|EnhancedInputActionSetTarget
  (params (ActionValue :type Boolean) (ElapsedSeconds :type Float%20%28double-precision%29) (TriggeredSeconds :type Float%20%28double-precision%29) (InputAction :type Input%20Action%20Object%20Reference :default "/Game/Characters/Creature/Input/Actions/SetTarget.SetTarget"))
  ;[1 1 1] SetTarget
  (:Triggered
    (Class|Mostriciattolo5Character|FindCharactertoTarget (Class|Actor|GetInputAxisKeyValue))))

(event Input|KeyboardEvents|Q
  (params (Key :type Key%20Structure))
  ;[1 1 1] Change Target Left/Right
  (:Pressed
    (Class|Mostriciattolo5Character|FindCharactertoTarget -1.0)))

(event Input|KeyboardEvents|E
  (params (Key :type Key%20Structure))
  ;[1 1 1] Change Target Left/Right
  (:Pressed
    (Class|Mostriciattolo5Character|FindCharactertoTarget 1.0)))

(event Custom|BP_FrontPossess
  (params (CatchingCharacter :type Character%20Object%20Reference))
  (|FrontalPossession_2 CatchingCharacter))

(event Custom|CameraArmForDepossession
  (bind _satrack (Timeline|SpringArmTimeline PlayFromStart)
    (:Update
      (Variables|/Script/Engine.SpringArmComponent|SetTargetArmLength (Variables|Default|GetSpringArm) _satrack)
      (Pawn|SetControlRotation (Game|GetPlayerController 0) (Math|Rotator|MakeRotator 0.0 -3e+01 (.yaw (Pawn|GetControlRotation :!class /Script/Engine.Pawn)))))))

(event Custom|PossessProva
  ;[0.3219 1 0] Possessione
  (|Possession))

(event EventAfterDepossessed
  (params (Possessor :type Mostriciattolo%205%20Player%20Object%20Reference))
  ;[1 0.007126 0] Depossessione
  (|Depossession))

(event EventPossessFront
  ;[1 0.3394 0] Possessione Frontale
  (|FrontalPossession))

(event EventTurnCameratoTarget
  (bind _returnvalue (Class|Mostriciattolo5Character|GetCurrentFocus))
  (bind _springarm (Variables|Default|GetSpringArm))
  (bind _returnvalue_2 (Transformation|GetWorldLocation _springarm))
  (bind _returnvalue_3 (Transformation|GetActorLocation _returnvalue))
  (bind _returnvalue_4 (Math|Rotator|FindLookatRotation _returnvalue_2 _returnvalue_3))
  ;[0.2292 0.2292 0.2292] turn camera to target
  (Pawn|SetControlRotation (Game|GetPlayerController 0) (Math|Rotator|MakeRotator 0.0 (+ (.pitch _returnvalue_4) -1e+01) (.yaw _returnvalue_4))))

(event EventLocktoPossessSocket
  (params (Target :type Mostriciattolo%205%20Character%20Object%20Reference)))

(event EventAttachAnimation
  ;[0.3219 1 0] Possessione
  (|Possession))

(event Custom|OnFinished_Event
  (Class|Mostriciattolo5Player|ControllNPCDelayed))

(event Custom|OnFinishedCustomEvent
  ;[0 1 0.1927] WIN
  (Class|Mostriciattolo5Player|ControllNPCDelayed))

(event EventTapKeyPassedScript
  ;[0 1 0.1927] WIN
  (bind _returnvalue (Animation|PlayAnimMontage "/Game/Characters/Creature/Animations/QTE/QTE_Creature_PossessFrontal_Montage.QTE_Creature_PossessFrontal_Montage" 1.0 "Win"))
  (Animation|PlayAnimMontage (stale _returnvalue) "/Game/Characters/Creature/Animations/QTE/QTE_NPC_PossessFrontal_Montage.QTE_NPC_PossessFrontal_Montage" 1.0 "Win")
  (bind _returnvalue_2 (Sequencer|Player|CreateLevelSequencePlayer "/Game/Sequencer/Seq_FrontalPossession_Win.Seq_FrontalPossession_Win" (Utilities|Struct|MakeMovieSceneSequencePlaybackSettings true "(Value=0)" 1.0 0.0 false false false false false false false false)))
  (Utilities|FlowControl|Delay 1.0)
  (Audio|PlaySound2D "/Game/Effects/Sounds/Voice/Guards/FrontalPossession/SFX_Guard_FrontalPoss_Lose.SFX_Guard_FrontalPoss_Lose" 1.0 1.0 0.0 0 0)
  (Utilities|FlowControl|Delay 0.8)
  (Audio|PlaySound2D "/Game/Effects/Sounds/Creature/LongPossess.LongPossess" 0.9 1.0 0.0 0 0)
  (EventDispatchers|AssignOnFinished _returnvalue_2 (delegate Custom|OnFinishedCustomEvent))
  (|ResetCameraPosition_2)
  (Utilities|FlowControl|Delay _returnvalue)
  (bind _returnvalue_3 (Class|Mostriciattolo5Player|GetCurrentPossessed))
  (Class|BPICharacter|ResetBehaviorAlert(Message) _returnvalue_3)
  ;;[1 1 1] il png puo mirare in alto
  (Variables|/Script/Engine.PlayerCameraManager|SetViewPitchMax (Variables|/Script/Engine.PlayerController|GetPlayerCameraManager (Game|GetPlayerController 0)) 5e+01))

(event EventTapKeyFailedScript
  ;[1 0.007126 0] Lose
  (Animation|PlayAnimMontage "/Game/Characters/Creature/Animations/QTE/QTE_Creature_PossessFrontal_Montage.QTE_Creature_PossessFrontal_Montage" 1.0 "Lose")
  (Animation|PlayAnimMontage (stale _returnvalue) "/Game/Characters/Creature/Animations/QTE/QTE_NPC_PossessFrontal_Lose_Montage.QTE_NPC_PossessFrontal_Lose_Montage" 1.0 "Lose")
  (Sequencer|Player|CreateLevelSequencePlayer "/Game/Sequencer/Seq_FrontalPossession_Lose.Seq_FrontalPossession_Lose" (Utilities|Struct|MakeMovieSceneSequencePlaybackSettings true "(Value=0)" 1.0 0.0 false false false false false false false false))
  (Utilities|FlowControl|Delay 1.2)
  (Audio|PlaySound2D "/Game/Effects/Sounds/Voice/Guards/FrontalPossession/SFX_Guard_FrontalWin.SFX_Guard_FrontalWin" 1.0 1.0 0.0 0 0))

(fn GetIsDead
  (return false))

(fn GetIsTarget
  (return (Variables|Default|GetCanBeTarget)))