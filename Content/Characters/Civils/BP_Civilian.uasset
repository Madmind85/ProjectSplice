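; Civilian NPC character that reacts when it sees a pawn tagged Mostriciattolo (little monster).
; Its PawnSensing event triggers a one-time scared montage on first sighting, waits out its length, then sets MostriciattoloMet and writes the Mostriciattolo blackboard key with no object wired.
; Sightings after that flag is set write the seen pawn to that key, passing the target to the AI's blackboard.
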(event OnSeePawn(PawnSensing)
  (params (Pawn :type Pawn%20Object%20Reference))
  (if (Actor|ActorHasTag Pawn "Mostriciattolo")
    (if (Variables|Default|GetMostriciattoloMet)
      (AI|Components|Blackboard|SetValueasObject (AI|GetBlackboard 0) (Variables|Default|GetMostriciattolo) Pawn)
      (else
        (Utilities|FlowControl|DoOnce false
          (:Completed
            (bind _returnvalue (Animation|PlayAnimMontage "/Game/Characters/Enemies/Animations/ANIM_NPC_Scared_Montage.ANIM_NPC_Scared_Montage" 1.0 "None"))
            (Utilities|FlowControl|Delay _returnvalue)
            (Variables|Default|SetMostriciattoloMet true)
            (AI|Components|Blackboard|SetValueasObject (AI|GetBlackboard 0) (Variables|Default|GetMostriciattolo) 0)))))))

(event EventBeginPlay
  (|CallParentFunction) ; This node is disabled and will not be called.\nDrag off pins to build functionality.
)

(event Collision|EventActorBeginOverlap
  (params (OtherActor :type Actor%20Object%20Reference)))

(event EventTick
  (params (DeltaSeconds :type Float%20%28single-precision%29))
  (|CallParentFunction DeltaSeconds) ; This node is disabled and will not be called.\nDrag off pins to build functionality.
)

(fn ConstructionScript
  (|CallParentFunction))