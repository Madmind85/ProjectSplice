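; Civilian NPC character that detects the player's creature (Mostriciattolo) and can be possessed and controlled by it.
; Pawn sensing and an inner-cone check drive alert or aggressive blackboard status through BPBehaviourComponent, with a per-tick lost-target reset.
; Possession events toggle the creature's collision and reset status; depossession detaches it and restarts the behavior tree.
; While possessed, Enhanced Input drives movement, camera lean, aiming, attack and target selection, with camera focus tracking.
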(event OnSeePawn(PawnSensing)
  (params (Pawn :type Pawn%20Object%20Reference))
  (CallFunction|OnMostriciattoloSeen Pawn))

(event Custom|NextTargetPont
  (Default|SetNextTarget (Variables|Default|GetBP_BehaviourComponent)))

(event Input|EnhancedActionEvents|EnhancedInputActionIA_Move_Forward
  (params (ActionValue :type Float%20%28double-precision%29) (ElapsedSeconds :type Float%20%28double-precision%29) (TriggeredSeconds :type Float%20%28double-precision%29) (InputAction :type Input%20Action%20Object%20Reference :default "/Game/ThirdPerson/Input/Actions/IA_Move_Forward.IA_Move_Forward"))
  ;[1 1 1] Roba de locomotion - INPUT
  (:Triggered
    (goto _label Triggered))
  (:Started
    (Utilities|MoveForwardAction ActionValue TriggeredSeconds :!label _label))
  (:Completed
    (goto _label Finished)))

(event Input|EnhancedActionEvents|EnhancedInputActionIA_Move_Right
  (params (ActionValue :type Float%20%28double-precision%29) (ElapsedSeconds :type Float%20%28double-precision%29) (TriggeredSeconds :type Float%20%28double-precision%29) (InputAction :type Input%20Action%20Object%20Reference :default "/Game/ThirdPerson/Input/Actions/IA_Move_Right.IA_Move_Right"))
  ;[1 1 1] Roba de locomotion - INPUT
  (:Triggered
    (goto _label Triggered))
  (:Started
    (Utilities|MoveRightAction ActionValue TriggeredSeconds :!label _label))
  (:Completed
    (goto _label Finished)))

(event Input|EnhancedActionEvents|EnhancedInputActionIA_JogOverride
  (params (ActionValue :type Boolean) (ElapsedSeconds :type Float%20%28double-precision%29) (TriggeredSeconds :type Float%20%28double-precision%29) (InputAction :type Input%20Action%20Object%20Reference :default "/Game/ThirdPerson/Input/Actions/IA_JogOverride.IA_JogOverride"))
  ;[1 1 1] Roba de locomotion - INPUT
  (:Triggered
    (goto _label Triggered))
  (:Started
    (Utilities|JogOverrideAction ActionValue :!label _label))
  (:Completed
    (goto _label Finished)))

(event Input|EnhancedActionEvents|EnhancedInputActionIA_LookUP
  (params (ActionValue :type Float%20%28double-precision%29) (ElapsedSeconds :type Float%20%28double-precision%29) (TriggeredSeconds :type Float%20%28double-precision%29) (InputAction :type Input%20Action%20Object%20Reference :default "/Game/ThirdPerson/Input/Actions/IA_LookUP.IA_LookUP"))
  ;[1 1 1] Roba de locomotion - INPUT
  (:Triggered
    (Input|HandleLookUpInput ActionValue)))

(event Input|EnhancedActionEvents|EnhancedInputActionIA_LookTurn
  (params (ActionValue :type Float%20%28double-precision%29) (ElapsedSeconds :type Float%20%28double-precision%29) (TriggeredSeconds :type Float%20%28double-precision%29) (InputAction :type Input%20Action%20Object%20Reference :default "/Game/ThirdPerson/Input/Actions/IA_LookTurn.IA_LookTurn"))
  ;[1 1 1] Roba de locomotion - INPUT
  (:Triggered
    (Input|HandleTurnInput ActionValue)))

(event EventBeginPlay
  ;[1 0.3473 0.2776] BaginPlay
  (Class|KLSLocomotionBlueprintLibrary|TryLinkAnimLayer (Variables|Character|GetMesh) "/Game/Characters/Enemies/KLS_ABP_Linked_Enemies.KLS_ABP_Linked_Enemies_C" false "None")
  (CallFunction|LeanCamera)
  (Variables|Default|SetSelectTargetArrow (Variables|Default|GetSelectTarget)))

(event EventPossessed
  (params (NewController :type Controller%20Object%20Reference))
  ;[1 1 1] Roba de locomotion - INPUT
  (bind _asplayer_controller (Utilities|Casting|CastToPlayerController NewController))
  (Input|AddMappingContext (PlayerController|LocalPlayerSubsystems|GetEnhancedInputLocalPlayerSubsystem _asplayer_controller) "/Game/ThirdPerson/Input/InputMappingContext.InputMappingContext" 0 "(bIgnoreAllPressedKeysUntilRelease=True,bForceImmediately=False)"))

(event EventTick
  (params (DeltaSeconds :type Float%20%28single-precision%29))
  (Utilities|FlowControl|Sequence
    (:then_0
      (CallFunction|TargetNotFoundCheck))
    (:then_1
      (Rendering|SetVisibility (Variables|Default|GetAttentoMesh) (== (Class|BlackboardComponent|GetValueasEnum (AI|GetBlackboard 0) (Variables|/Game/Components/BP_BehaviourComponent.BP_BehaviourComponent_C|GetCurrentStatus (Variables|Default|GetBP_BehaviourComponent))) 1) false))
    (:then_2
      (if (Variables|Default|GetCanRotateTowardsPlayer)
        (Class|Mostriciattolo5Character|RotatePlayerTowardsTarget (Variables|Default|GetTarget))))))

(fn ConstructionScript)

(fn EnemySpotted
  (params (Mostriciattolo :type Object%20Object%20Reference))
  (bind _output_get (Variables|Default|SetCurrentNPCStatus "Aggressivo"))
  (Default|SetMostriciattoloonBB (Variables|Default|GetBP_BehaviourComponent) Mostriciattolo true _output_get)
  (Variables|/Script/Engine.CharacterMovementComponent|SetMaxWalkSpeed (Variables|Character|GetCharacterMovement) 6e+02))

(fn TargetNotFoundCheck
  (bind _returnvalue (Class|Mostriciattolo5Character|HasLostTarget))
  (if _returnvalue
    (if (!= (Class|BlackboardComponent|GetValueasEnum (AI|GetBlackboard 0) (Variables|/Game/Components/BP_BehaviourComponent.BP_BehaviourComponent_C|GetCurrentStatus (Variables|Default|GetBP_BehaviourComponent))) 1)
      (Default|SetMostriciattoloonBB (Variables|Default|GetBP_BehaviourComponent) 0 false)
      (Variables|/Script/Engine.CharacterMovementComponent|SetMaxWalkSpeed (Variables|Character|GetCharacterMovement) 147.0))))

(fn CheckOuterConeContact
  (if (>= (Utilities|Time|GetTimeSeconds) (+ (Variables|Default|GetResetOuterConeTime) (Variables|Default|GetOuterConeTimeCount)))
    _))

(fn OnMostriciattoloSeen
  (params (Mostriciattolo :type Object%20Object%20Reference))
  (bind _asmostriciattolo_5character (Utilities|Casting|CastToMostriciattolo5Character Mostriciattolo))
  (if (Variables|/Script/Mostriciattolo5.Mostriciattolo5Character|GetIsTarget _asmostriciattolo_5character)
    (bind _returnvalue (CallFunction|CheckInnerCon _asmostriciattolo_5character))
    (if _returnvalue
      (CallFunction|EnemySpotted _asmostriciattolo_5character)
      (Variables|Default|SetTargetLastSeen (Utilities|Time|GetTimeSeconds))
      (else
        (Default|SetNPCtoAttento (Variables|Default|GetBP_BehaviourComponent) _asmostriciattolo_5character 1)
        (Variables|Default|SetTargetLastSeen (Utilities|Time|GetTimeSeconds))))
    (else
      ;[1 1 1] controlla se l'npc è stato appena posseduto(can be target che si resetta dopo notargettime secondi) ed eventualmente lo setta come target
      (if (Variables|/Script/Mostriciattolo5.Mostriciattolo5Character|GetCanBeTarget _asmostriciattolo_5character)
        (Variables|/Script/Mostriciattolo5.Mostriciattolo5Character|SetIsTarget _asmostriciattolo_5character true)))))

(fn SetCollisiononMostriciattolo
  (params (CollisionOn :type Boolean) (Mostriciattolo :type Mostriciattolo%205%20Player%20Object%20Reference))
  (if CollisionOn
    (Collision|SetCollisionEnabled (Variables|/Script/Engine.Character|GetMesh Mostriciattolo) "QueryAndProbe")
    (Collision|SetCollisionEnabled (Variables|/Script/Engine.Character|GetCapsuleComponent Mostriciattolo) "QueryAndProbe")
    (else
      (Collision|SetCollisionEnabled (Variables|/Script/Engine.Character|GetMesh Mostriciattolo) "NoCollision")
      (Collision|SetCollisionEnabled (Variables|/Script/Engine.Character|GetCapsuleComponent Mostriciattolo) "NoCollision"))))

(fn BPCheckInnerCon
  (params (CharacterInSight :type Mostriciattolo%205%20Character%20Object%20Reference))
  (bind _returnvalue (Class|Mostriciattolo5Character|CheckInnerSightAngle CharacterInSight (Variables|/Script/AIModule.PawnSensingComponent|GetSightRadius (Variables|Default|GetPawnSensing))))
  (return _returnvalue))

(fn ChangeCameraShoulder
  (params (New%20Location%20Y :type Float%20%28double-precision%29))
  (Variables|/Script/Engine.SpringArmComponent|SetSocketOffset (Variables|Default|GetSpringArm) (Math|Vector|MakeVector 0.0 New%20Location%20Y 0.0)))

(fn HandleForwardInput
  (params (Input%20Value :type Float%20%28double-precision%29))
  (Pawn|Input|AddMovementInput (Math|Vector|GetForwardVector (Math|Rotator|MakeRotator 0.0 0.0 (.yaw (Pawn|GetControlRotation :!class /Script/Engine.Pawn)))) Input%20Value false))

(fn HandleRightwardInput
  (params (InputValue :type Float%20%28double-precision%29))
  (Pawn|Input|AddMovementInput (Math|Vector|GetRightVector (Math|Rotator|MakeRotator 0.0 0.0 (.yaw (Pawn|GetControlRotation :!class /Script/Engine.Pawn)))) InputValue false))

(fn HandleLookUpInput
  (params (InputValue :type Float%20%28double-precision%29))
  (Pawn|Input|AddControllerPitchInput InputValue))

(fn HandleTurnInput
  (params (InputValue :type Float%20%28double-precision%29))
  (Pawn|Input|AddControllerYawInput InputValue))

(fn GetMovementSpeed
  (bind _returnvalue (Math|Float|MakeLiteralFloat 0.586))
  (bind _ia_move_forward_action_value (Variables|Default|GetIA%20Move%20Forward%20Action%20Value))
  (bind _ia_move_right_action_value (Variables|Default|GetIA%20Move%20Right%20Action%20Value))
  (bind _returnvalue_2 (Math|Vector|MakeVector _ia_move_forward_action_value _ia_move_right_action_value 0.0))
  (bind _returnvalue_3 (Math|Float|Absolute(Float) _returnvalue))
  (bind _returnvalue_4 (Math|Vector|VectorLength _returnvalue_2))
  (bind _returnvalue_5 (Math|Vector|ClampVectorSize _returnvalue_2 0.207 0.332))
  (bind _returnvalue_6 (Math|Float|Absolute(Float) _returnvalue_4))
  (bind _returnvalue_7 (< _returnvalue_6 _returnvalue_3))
  (bind _returnvalue_8 (Math|Vector|SelectVector _returnvalue_5 _returnvalue_2 _returnvalue_7))
  (bind (_x _y) (Math|Vector|BreakVector _returnvalue_8))
  (return _x _y))

(fn SetCanRotatetoPlayer
  (params (Target :type Mostriciattolo%205%20Character%20Object%20Reference) (CanRotateTowardsPlayer :type Boolean))
  (Variables|Default|SetCanRotateTowardsPlayer CanRotateTowardsPlayer)
  (Variables|Default|SetTarget Target))

(event EventAfterPossession
  (params (Possessor :type Mostriciattolo%205%20Player%20Object%20Reference))
  (Input|DisableInput (Game|GetPlayerController 0))
  (CallFunction|SetCollisiononMostriciattolo false Possessor)
  (bind _output_get (Variables|Default|SetCurrentNPCStatus "Tranquillo"))
  (Default|SetMostriciattoloonBB (Variables|Default|GetBP_BehaviourComponent) 0 false _output_get)
  (Utilities|FlowControl|Delay 0.4)
  (Variables|Default|SetCanBeTarget false)
  (Utilities|FlowControl|Delay 0.4)
  (Input|EnableInput (Game|GetPlayerController 0)))

(event EventAfterDepossessed
  (params (Possessor :type Mostriciattolo%205%20Player%20Object%20Reference))
  (Default|RestartBT (Variables|Default|GetBP_BehaviourComponent) self)
  (Transformation|DetachFromComponent (Variables|/Script/Engine.Character|GetCapsuleComponent Possessor) "KeepWorld" "KeepWorld" "KeepWorld" true)
  (CallFunction|SetCollisiononMostriciattolo true Possessor)
  (Input|EnableInput Possessor (Game|GetPlayerController 0))
  (Class|SkeletalMeshComponent|SetAnimClass (Variables|Character|GetMesh) "/Game/Characters/Enemies/KLS_ABP_Enemies.KLS_ABP_Enemies_C"))

(event EventSetTarget
  (Development|SetHiddeninGame (Variables|Default|GetTargetArrow1) false false)
  ;[1 1 1] cambiare perchè sia universale
  (bind _asbp_mostriciattolo (Utilities|Casting|CastToBP_Mostriciattolo (Game|GetPlayerCharacter 0)))
  (Variables|/Script/CinematicCamera.CineCameraComponent|SetFocusSettings (Variables|/Game/ThirdPerson/Blueprints/BP_Mostriciattolo.BP_Mostriciattolo_C|GetCineCameraCreature _asbp_mostriciattolo) (Utilities|Struct|MakeCameraFocusSettings "Tracking" 0.0 (Utilities|Struct|MakeCameraTrackingFocusSettings (Utilities|ResolveSoftReference self) "0.000000,0.000000,0.000000" true) true 0.5 0.0)))

(event EventTurnCameratoTarget
  (bind _returnvalue (Class|Mostriciattolo5Character|GetCurrentFocus))
  (Pawn|SetControlRotation (Game|GetPlayerController 0) (Math|Rotator|MakeRotator 0.0 (+ (.pitch (Math|Rotator|FindLookatRotation (Transformation|GetWorldLocation (Variables|Default|GetSpringArm)) (Transformation|GetActorLocation _returnvalue))) 2.0) (.yaw (Math|Rotator|FindLookatRotation (Transformation|GetWorldLocation (Variables|Default|GetSpringArm)) (Transformation|GetActorLocation _returnvalue)))))
  (Transformation|SetActorRotation (Math|Rotator|MakeRotator 0.0 0.0 (.yaw (Transformation|GetActorRotation)))))

(event EventStopMovement
  (Default|StopBT (Variables|Default|GetBP_BehaviourComponent)))

(event EventResetTarget
  (Development|SetHiddeninGame (Variables|Default|GetTargetArrow1) true false)
  ;[1 1 1] cambiare perchè sia universale
  (bind _asbp_mostriciattolo (Utilities|Casting|CastToBP_Mostriciattolo (Game|GetPlayerCharacter 0)))
  (Variables|/Script/CinematicCamera.CineCameraComponent|SetFocusSettings (Variables|/Game/ThirdPerson/Blueprints/BP_Mostriciattolo.BP_Mostriciattolo_C|GetCineCameraCreature _asbp_mostriciattolo) (Utilities|Struct|MakeCameraFocusSettings "Manual" 1e+02 (Utilities|Struct|MakeCameraTrackingFocusSettings 0 "0.000000,0.000000,0.000000" false) true 0.5 0.0)))

(event Custom|LeanCamera
  (Utilities|FlowControl|FlipFlop
    (:A
      (Class|ValueOverTimeComponent|StartCameraMoveOverTime (Variables|Default|GetBP_ValueOverTimeComponent) false))
    (:B
      (Class|ValueOverTimeComponent|StartCameraMoveOverTime (Variables|Default|GetBP_ValueOverTimeComponent) true))))

(event Input|EnhancedActionEvents|EnhancedInputActionCrouch
  (params (ActionValue :type Boolean) (ElapsedSeconds :type Float%20%28double-precision%29) (TriggeredSeconds :type Float%20%28double-precision%29) (InputAction :type Input%20Action%20Object%20Reference :default "/Game/ThirdPerson/Input/Actions/Crouch.Crouch"))
  (:Triggered
    (Character|Crouch))
  (:Completed
    (Character|UnCrouch)))

(event Input|EnhancedActionEvents|EnhancedInputActionCameraLean
  (params (ActionValue :type Boolean) (ElapsedSeconds :type Float%20%28double-precision%29) (TriggeredSeconds :type Float%20%28double-precision%29) (InputAction :type Input%20Action%20Object%20Reference :default "/Game/ThirdPerson/Input/Actions/CameraLean.CameraLean"))
  (:Triggered
    (CallFunction|LeanCamera)))

(event Input|EnhancedActionEvents|EnhancedInputActionToggleSelectMode
  (params (ActionValue :type Boolean) (ElapsedSeconds :type Float%20%28double-precision%29) (TriggeredSeconds :type Float%20%28double-precision%29) (InputAction :type Input%20Action%20Object%20Reference :default "/Game/ThirdPerson/Input/Actions/ToggleSelectMode.ToggleSelectMode"))
  (:Triggered
    (Class|Mostriciattolo5Character|StartSelectFocusMode)))

(event Input|EnhancedActionEvents|EnhancedInputActionIA_JogOverride
  (params (ActionValue :type Boolean) (ElapsedSeconds :type Float%20%28double-precision%29) (TriggeredSeconds :type Float%20%28double-precision%29) (InputAction :type Input%20Action%20Object%20Reference :default "/Game/ThirdPerson/Input/Actions/IA_JogOverride.IA_JogOverride"))
  (:Triggered
    (Variables|/Script/Engine.CharacterMovementComponent|SetMaxWalkSpeed (Variables|Character|GetCharacterMovement) 6e+02))
  (:Canceled
    (Variables|/Script/Engine.CharacterMovementComponent|SetMaxWalkSpeed (Variables|Character|GetCharacterMovement) 147.0 :!label _label))
  (:Completed
    (goto _label)))

(event Input|EnhancedActionEvents|EnhancedInputActionPossess
  (params (ActionValue :type Boolean) (ElapsedSeconds :type Float%20%28double-precision%29) (TriggeredSeconds :type Float%20%28double-precision%29) (InputAction :type Input%20Action%20Object%20Reference :default "/Game/ThirdPerson/Input/Actions/Possess.Possess"))
  (:Started
    (Class|Mostriciattolo5Character|Depossess)))

(event Input|EnhancedActionEvents|EnhancedInputActionIA_Aim
  (params (ActionValue :type Boolean) (ElapsedSeconds :type Float%20%28double-precision%29) (TriggeredSeconds :type Float%20%28double-precision%29) (InputAction :type Input%20Action%20Object%20Reference :default "/Game/ThirdPerson/Input/Actions/IA_Aim.IA_Aim"))
  (:Triggered
    (bind _asklscharacter_movement_component (Utilities|Casting|CastToKLSCharacterMovementComponent (Variables|Character|GetCharacterMovement)))
    (Class|KLSCharacterMovementComponent|ToggleAiming _asklscharacter_movement_component true))
  (:Completed
    (bind _asklscharacter_movement_component_2 (Utilities|Casting|CastToKLSCharacterMovementComponent (Variables|Character|GetCharacterMovement)))
    (Class|KLSCharacterMovementComponent|ToggleAiming _asklscharacter_movement_component_2 false)))

(event Input|EnhancedActionEvents|EnhancedInputActionIA_Attack
  (params (ActionValue :type Boolean) (ElapsedSeconds :type Float%20%28double-precision%29) (TriggeredSeconds :type Float%20%28double-precision%29) (InputAction :type Input%20Action%20Object%20Reference :default "/Game/ThirdPerson/Input/Actions/IA_Attack.IA_Attack"))
  (:Started
    (Class|Mostriciattolo5Character|Attack)
    ;[1 1 1] ovviamente dqa cambiare
    (Audio|PlaySoundatLocation "/Game/Effects/Audio/Shot_Cue.Shot_Cue" (Transformation|GetActorLocation) "0, 0, 0" 1.0 1.0 0.0 0 0 0 0)))

(event Input|KeyboardEvents|Q
  (params (Key :type Key%20Structure))
  (:Pressed
    (Class|Mostriciattolo5Character|FindCharactertoTarget -1.0)))

(event Input|KeyboardEvents|E
  (params (Key :type Key%20Structure))
  (:Pressed
    (Class|Mostriciattolo5Character|FindCharactertoTarget 1.0)))