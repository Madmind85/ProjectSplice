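; BP_ArmorBase is a base actor for enemy armor pieces that can detach from their owner character and fall as physics objects.
; On BeginPlay it disables simulation, then calls SetRandomMesh on its skeletal mesh after a short delay.
; SetPhysics waits briefly, detaches the piece in world space, enables collision and physics, removes its socket entry from the owner's ArmorParts, and prints a debug message.
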(event EventSetPhysics
  (Utilities|FlowControl|Delay 0.12)
  (Transformation|DetachFromActor "KeepWorld" "KeepWorld" "KeepWorld")
  (Collision|SetCollisionEnabled (Variables|Default|GetSkeletalMesh) "QueryAndPhysics")
  (Physics|SetSimulatePhysics (Variables|Default|GetSkeletalMesh) true)
  (Utilities|Map|Remove (Variables|/Script/Mostriciattolo5.Mostriciattolo5Character|GetArmorParts (Variables|Default|GetOwnerChar)) (Variables|Default|GetAttchSocketName))
  (Development|PrintString (Utilities|String|Append (Utilities|GetDisplayName self) "phisics enabled") true true "(R=0.000000,G=0.660000,B=1.000000,A=1.000000)" 1e+01))

(event Collision|EventActorBeginOverlap
  (params (OtherActor :type Actor%20Object%20Reference)))

(event EventTick
  (params (DeltaSeconds :type Float%20%28single-precision%29)))

(event EventBeginPlay
  (Physics|SetSimulatePhysics (Variables|Default|GetSkeletalMesh) false)
  (Utilities|FlowControl|Delay 0.2)
  (Class|Armor|SetRandomMesh (Variables|Default|GetSkeletalMesh)))

(fn ConstructionScript)