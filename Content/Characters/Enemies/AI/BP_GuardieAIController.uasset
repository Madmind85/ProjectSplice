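; AI controller for the Guardie enemy that handles its perception updates, alert voice sounds and shutdown on death.
; It sets up the BB_Guardie blackboard on BeginPlay and forwards AI perception updates to OnActorSeen, whose logic is not in this graph.
; Voice events select a sound by stimulus name, such as sight, hearing or a found corpse, and play it at the pawn's location.
; The death function deactivates AI perception.
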(event OnPerceptionUpdated(AIPerception)
  (params (UpdatedActors :type Array%20of%20Actor%20Object%20References))
  (Class|MostriciattoloAIController|OnActorSeen UpdatedActors))

(event EventBeginPlay
  (Class|AIController|UseBlackboard "/Game/Characters/Enemies/AI/BB_Guardie.BB_Guardie"))

(event EventTick
  (params (DeltaSeconds :type Float%20%28single-precision%29)))

(event EventVoiceFX
  (params (VoiceName :type Name :default "None"))
  (CallFunction|VoiceSoundSelect VoiceName))

(fn ConstructionScript)

(fn BPonDeathController
  (Components|Activation|Deactivate (Variables|Default|GetAIPerception)))

(fn BPVoiceSoundSelect
  (params (VoiceName :type Name))
  (Variables|Default|SetVoiceLocation (Transformation|GetActorLocation (Pawn|GetControlledPawn)))
  (switch name VoiceName
    (:PeripheralSight
      (Audio|PlaySoundatLocation "/Game/Effects/Sounds/Voice/Guards/SFX_Vis_03.SFX_Vis_03" (Variables|Default|GetVoiceLocation) "0, 0, 0" 1.0 1.0 0.0 0 0 0 0))
    (:Hearing
      (Audio|PlaySoundatLocation "/Game/Effects/Sounds/Voice/Guards/SFX_Ear_01.SFX_Ear_01" (Variables|Default|GetVoiceLocation) "0, 0, 0" 1.0 1.0 0.0 0 0 0 0 :!label _label))
    (:ShootHearing
      (goto _label))
    (:CorpseSight
      (Audio|PlaySoundatLocation "/Game/Effects/Sounds/Voice/Guards/SFX_BodyFound_02.SFX_BodyFound_02" (Variables|Default|GetVoiceLocation) "0, 0, 0" 1.0 1.0 0.0 0 0 0 0))
    (:MonsterSight
      (Audio|PlaySoundatLocation "/Game/Effects/Sounds/Voice/Guards/Alert/SFX_GuardAlert_Cue.SFX_GuardAlert_Cue" (Variables|Default|GetVoiceLocation) "0, 0, 0" 1.0 1.0 0.0 0 0 0 0 :!label _label_2))
    (:GuardSight
      (goto _label_2))))