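; Grinding effect actor that shows Niagara sparks and smoke while it is in contact with a surface.
; Each tick a short downward sphere trace activates the effect and aligns it to the hit normal, or deactivates it when nothing is hit.
; A resettable DoOnce starts playback, likely audio, once per contact, and losing contact stops it.
; The construction script applies the exposed point light settings and spark and smoke color parameters.
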(event EventTick
  (params (DeltaSeconds :type Float%20%28single-precision%29))
  (bind _returnvalue (Transformation|GetWorldLocation))
  (bind _ns_grind (Variables|Default|GetNS_Grind))
  (bind _ns_grind_2 (Variables|Default|GetNS_Grind))
  (bind (_outhit _returnvalue_2) (Collision|SphereTraceForObjects _returnvalue (+ _returnvalue "0.000000,0.000000,-20.000000") 5e+01 (Utilities|Array|MakeArray "ObjectTypeQuery1" "ObjectTypeQuery2" "ObjectTypeQuery3" "ObjectTypeQuery4" "ObjectTypeQuery5" "ObjectTypeQuery6") false 0 "None"))
  (if _returnvalue_2
    (Transformation|SetWorldRotation _ns_grind_2 (Math|Rotator|MakeRotationfromAxes (.Normal (Collision|BreakHitResult _outhit)) "0, 0, 0" "0, 0, 0") false false)
    (Components|Activation|Activate _ns_grind_2 false)
    (Rendering|SetVisibility _ns_grind_2 (Variables|Default|GetLightOn) false)
    (|DoOnceMultiInput :!label _label
      (:A%20Out
        (Audio|Components|Audio|Play 0.0)
        (Audio|Components|Audio|Play 0.0)))
    (else
      (Utilities|FlowControl|Sequence
        (:then_0
          (goto _label Reset%20In))
        (:then_1
          (Components|Activation|Deactivate _ns_grind)
          (Rendering|SetVisibility _ns_grind (Variables|Default|GetLightOff) false)
          (Audio|Components|Audio|Stop))))))

(fn ConstructionScript
  (bind _ns_grind (Variables|Default|GetNS_Grind))
  (bind _light_weld (Variables|Default|GetLight_Weld))
  ;[1 1 1] Light Settings
  (Rendering|Components|Light|SetLightColor _light_weld (Variables|LightSettings|GetLight%20Color) true)
  (Rendering|Components|Light|SetIntensity _light_weld (Variables|LightSettings|GetLight%20Intensity))
  (Rendering|Lighting|SetAttenuationRadius _light_weld (Variables|LightSettings|GetAttenuation%20Radius))
  (Rendering|Components|Light|SetCastShadows _light_weld (Variables|LightSettings|GetCast%20Shadows))
  (Transformation|AddRelativeLocation _light_weld (Variables|LightSettings|GetPoint%20Light%20Loc) false false)
  (Rendering|Components|Light|SetLightFunctionMaterial _light_weld (Variables|Default|GetLight%20Function%20Material))
  ;[1 1 1] Effect color Settings
  (Effects|Components|ParticleSystem|SetColorParameter _ns_grind "SparkColor" (Variables|EffectSettings|GetSpark%20Color))
  (Effects|Components|ParticleSystem|SetFloatParameter _ns_grind "SparkColorScale" (Variables|EffectSettings|GetSparkIntensity))
  (Effects|Components|ParticleSystem|SetFloatParameter _ns_grind "SparkAlphaScale" (Variables|EffectSettings|GetSpark%20Alpha%20Intensity))
  (Effects|Components|ParticleSystem|SetColorParameter _ns_grind "SmokeColor" (Variables|EffectSettings|GetSmoke%20Color))
  (Effects|Components|ParticleSystem|SetFloatParameter _ns_grind "SmokeColorScale" (Variables|EffectSettings|GetSmoke%20Color%20Intensity))
  (Effects|Components|ParticleSystem|SetFloatParameter _ns_grind "SmokeAlphaScale" (Variables|EffectSettings|GetSmoke%20Alpha%20Intensity)))