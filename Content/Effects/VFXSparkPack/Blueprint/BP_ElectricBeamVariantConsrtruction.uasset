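; Electric arc effect actor that throws three randomly aimed beams from its particle component onto nearby surfaces.
; A looping timer, its interval randomized once at BeginPlay, calls ShootArc to fire three beam events, two with random retriggerable delays.
; Each line-traces to a random radial point; hits set beam targets, spawn tinted impacts and flash a light, while misses disable that emitter.
; Construction script configures core and impact lights plus beam color.
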(event Custom|CE_ShootArc
  (bind _vfx_beamtest (Variables|Default|GetVFX_BeamTest))
  (bind _returnvalue (Transformation|GetWorldLocation _vfx_beamtest))
  ;[1 1 1] Beam1
  (Class|ParticleSystemComponent|SetBeamSourcePoint 0 _returnvalue 1)
  (bind _output_get (Variables|Default|SetNewVar0 (* (Math|Random|RandomUnitVector) (Math|Random|RandomFloatinRange (Variables|EffectBehavior|GetBeam%20Radius%201%20Min) (Variables|EffectBehavior|GetBeam%20Radius%201%20Max)))))
  (Transformation|SetRelativeLocation (Variables|Default|GetDummyTarget) _output_get false false)
  (bind (_outhit _returnvalue_2) (Collision|LineTraceByChannel _returnvalue (Transformation|GetWorldLocation (Variables|Default|GetDummyTarget)) "TraceTypeQuery1" false 0 "None"))
  (if _returnvalue_2
    (Rendering|SetVisibility (Variables|Default|GetVFX_BeamTest) true false)
    (bind _returnvalue_3 (Effects|SpawnEmitteratLocation (Variables|EffectColorSettings|GetImpact%20Effect) (.Location (Collision|BreakHitResult _outhit)) (Math|Rotator|MakeRotationfromAxes (.Normal (Collision|BreakHitResult _outhit)) "0, 0, 0" "0, 0, 0")))
    (Effects|Components|ParticleSystem|SetColorParameter _returnvalue_3 "SparkColor" (Variables|EffectColorSettings|GetEffect%20Color))
    (Effects|Components|ParticleSystem|SetColorParameter _returnvalue_3 "SmokeColor" (Variables|EffectColorSettings|GetImpact%20Smoke%20Color))
    (Effects|Components|ParticleSystem|SetFloatParameter _returnvalue_3 "SparkColorScale" (Variables|EffectColorSettings|GetImpact%20Color%20Intensity))
    (Effects|Components|ParticleSystem|SetFloatParameter _returnvalue_3 "SparkAlpahaScale" (Variables|EffectColorSettings|GetImpact%20Alpha%20Scale))
    (Effects|Components|ParticleSystem|SetFloatParameter _returnvalue_3 "SmokeColorScale" (Variables|EffectColorSettings|GetImpact%20Smoke%20Color%20Intensity))
    (Effects|Components|ParticleSystem|SetFloatParameter _returnvalue_3 "SmokeAlphaScale" (Variables|EffectColorSettings|GetImpact%20Smoke%20AlphaScale))
    (Class|ParticleSystemComponent|SetBeamTargetPoint (Variables|Default|GetVFX_BeamTest) 0 (.Location (Collision|BreakHitResult _outhit)) 1)
    (Rendering|SetVisibility (Variables|Default|GetLightOn) false)
    (Transformation|SetWorldLocation (.Location (Collision|BreakHitResult _outhit)) false false)
    (Utilities|FlowControl|RetriggerableDelay 0.2)
    (Rendering|SetVisibility (Variables|Default|GetLightOff) false)
    (else
      (Class|ParticleSystemComponent|SetBeamTargetPoint 0 (Transformation|GetWorldLocation (Variables|Default|GetVFX_BeamTest)) 1)
      (Effects|Components|ParticleSystem|SetEmitterEnable (Variables|Default|GetVFX_BeamTest) "ElectricBeam0" false)
      (Rendering|SetVisibility (Variables|Default|GetLightOff) false))))

(event Custom|CE_ShootArc2
  (bind _vfx_beamtest (Variables|Default|GetVFX_BeamTest))
  (bind _returnvalue (Transformation|GetWorldLocation _vfx_beamtest))
  ;[1 1 1] beam2
  (Utilities|FlowControl|RetriggerableDelay (Math|Random|RandomFloatinRange 0.3 0.5))
  (Class|ParticleSystemComponent|SetBeamSourcePoint 1 _returnvalue 1)
  (bind _output_get (Variables|Default|SetNewVar0 (* (Math|Random|RandomUnitVector) (Math|Random|RandomFloatinRange (Variables|EffectBehavior|GetBeam%20Radius%202%20Min) (Variables|EffectBehavior|GetBeam%20Radius%202%20Max)))))
  (Transformation|SetRelativeLocation (Variables|Default|GetDummyTarget) _output_get false false)
  (bind (_outhit _returnvalue_2) (Collision|LineTraceByChannel _returnvalue (Transformation|GetWorldLocation (Variables|Default|GetDummyTarget)) "TraceTypeQuery1" false 0 "None"))
  (if _returnvalue_2
    (Rendering|SetVisibility (Variables|Default|GetVFX_BeamTest) true false)
    (bind _returnvalue_3 (Effects|SpawnEmitteratLocation (Variables|EffectColorSettings|GetImpact%20Effect) (.Location (Collision|BreakHitResult _outhit)) (Math|Rotator|MakeRotationfromAxes (.Normal (Collision|BreakHitResult _outhit)) "0, 0, 0" "0, 0, 0")))
    (Effects|Components|ParticleSystem|SetColorParameter _returnvalue_3 "SparkColor" (Variables|EffectColorSettings|GetEffect%20Color))
    (Effects|Components|ParticleSystem|SetColorParameter _returnvalue_3 "SmokeColor" (Variables|EffectColorSettings|GetImpact%20Smoke%20Color))
    (Effects|Components|ParticleSystem|SetFloatParameter _returnvalue_3 "SparkColorScale" (Variables|EffectColorSettings|GetImpact%20Color%20Intensity))
    (Effects|Components|ParticleSystem|SetFloatParameter _returnvalue_3 "SparkAlpahaScale" (Variables|EffectColorSettings|GetImpact%20Alpha%20Scale))
    (Effects|Components|ParticleSystem|SetFloatParameter _returnvalue_3 "SmokeColorScale" (Variables|EffectColorSettings|GetImpact%20Smoke%20Color%20Intensity))
    (Effects|Components|ParticleSystem|SetFloatParameter _returnvalue_3 "SmokeAlphaScale" (Variables|EffectColorSettings|GetImpact%20Smoke%20AlphaScale))
    (Class|ParticleSystemComponent|SetBeamTargetPoint (Variables|Default|GetVFX_BeamTest) 1 (.Location (Collision|BreakHitResult _outhit)) 1)
    (Rendering|SetVisibility (Variables|Default|GetLightOn) false)
    (Transformation|SetWorldLocation (.Location (Collision|BreakHitResult _outhit)) false false)
    (Utilities|FlowControl|RetriggerableDelay 0.2)
    (Rendering|SetVisibility (Variables|Default|GetLightOff) false)
    (else
      (Class|ParticleSystemComponent|SetBeamTargetPoint 1 (Transformation|GetWorldLocation (Variables|Default|GetVFX_BeamTest)) 1)
      (Effects|Components|ParticleSystem|SetEmitterEnable (Variables|Default|GetVFX_BeamTest) "ElectricBeam1" false)
      (Rendering|SetVisibility (Variables|Default|GetLightOff) false))))

(event Custom|CE_shootArc3
  (bind _vfx_beamtest (Variables|Default|GetVFX_BeamTest))
  (bind _returnvalue (Transformation|GetWorldLocation _vfx_beamtest))
  ;[1 1 1] beam3
  (Utilities|FlowControl|RetriggerableDelay (Math|Random|RandomFloatinRange 0.3 0.5))
  (Class|ParticleSystemComponent|SetBeamSourcePoint 2 _returnvalue 1)
  (bind _output_get (Variables|Default|SetNewVar0 (* (Math|Random|RandomUnitVector) (Math|Random|RandomFloatinRange (Variables|EffectBehavior|GetBeam%20Radius%203%20Min) (Variables|EffectBehavior|GetBeam%20Radius%203%20Max)))))
  (Transformation|SetRelativeLocation (Variables|Default|GetDummyTarget) _output_get false false)
  (bind (_outhit _returnvalue_2) (Collision|LineTraceByChannel _returnvalue (Transformation|GetWorldLocation (Variables|Default|GetDummyTarget)) "TraceTypeQuery1" false 0 "None"))
  (if _returnvalue_2
    (Rendering|SetVisibility (Variables|Default|GetVFX_BeamTest) true false)
    (bind _returnvalue_3 (Effects|SpawnEmitteratLocation (Variables|EffectColorSettings|GetImpact%20Effect) (.Location (Collision|BreakHitResult _outhit)) (Math|Rotator|MakeRotationfromAxes (.Normal (Collision|BreakHitResult _outhit)) "0, 0, 0" "0, 0, 0")))
    (Effects|Components|ParticleSystem|SetColorParameter _returnvalue_3 "SparkColor" (Variables|EffectColorSettings|GetEffect%20Color))
    (Effects|Components|ParticleSystem|SetColorParameter _returnvalue_3 "SmokeColor" (Variables|EffectColorSettings|GetImpact%20Smoke%20Color))
    (Effects|Components|ParticleSystem|SetFloatParameter _returnvalue_3 "SparkColorScale" (Variables|EffectColorSettings|GetImpact%20Color%20Intensity))
    (Effects|Components|ParticleSystem|SetFloatParameter _returnvalue_3 "SparkAlpahaScale" (Variables|EffectColorSettings|GetImpact%20Alpha%20Scale))
    (Effects|Components|ParticleSystem|SetFloatParameter _returnvalue_3 "SmokeColorScale" (Variables|EffectColorSettings|GetImpact%20Smoke%20Color%20Intensity))
    (Effects|Components|ParticleSystem|SetFloatParameter _returnvalue_3 "SmokeAlphaScale" (Variables|EffectColorSettings|GetImpact%20Smoke%20AlphaScale))
    (Class|ParticleSystemComponent|SetBeamTargetPoint (Variables|Default|GetVFX_BeamTest) 2 (.Location (Collision|BreakHitResult _outhit)) 1)
    (Rendering|SetVisibility (Variables|Default|GetLightOn) false)
    (Transformation|SetWorldLocation (.Location (Collision|BreakHitResult _outhit)) false false)
    (Utilities|FlowControl|RetriggerableDelay 0.2)
    (Rendering|SetVisibility (Variables|Default|GetLightOff) false)
    (else
      (Class|ParticleSystemComponent|SetBeamTargetPoint 2 (Transformation|GetWorldLocation (Variables|Default|GetVFX_BeamTest)) 1)
      (Effects|Components|ParticleSystem|SetEmitterEnable (Variables|Default|GetVFX_BeamTest) "ElectricBeam2" false)
      (Rendering|SetVisibility (Variables|Default|GetLightOff) false))))

(event EventBeginPlay
  ;[1 1 1] link to function
  (Utilities|Time|SetTimerbyFunctionName 0 "ShootArc" (Math|Random|RandomFloatinRange (Variables|EffectBehavior|GetBeam%20Time%20Min) (Variables|EffectBehavior|GetBeam%20Time%20Max)) true))

(fn ConstructionScript
  (bind _corelight (Variables|Default|GetCoreLight))
  (bind _vfx_beamtest (Variables|Default|GetVFX_BeamTest))
  (bind _impactlight (Variables|Default|GetImpactLight))
  ;[1 1 1] Core Light Settings
  (Rendering|Components|Light|SetLightColor _corelight (Variables|LightSettings|GetCore%20Light%20Color) true)
  (Rendering|Components|Light|SetIntensity _corelight (Variables|LightSettings|GetCore%20Light%20Intensity))
  (Rendering|Lighting|SetAttenuationRadius _corelight (Variables|LightSettings|GetCore%20Light%20Attenuation%20Radius))
  (Rendering|Components|Light|SetCastShadows _corelight (Variables|LightSettings|GetCore%20Light%20Cast%20Shadows))
  (Transformation|AddRelativeLocation _corelight (Variables|LightSettings|GetCore%20Light%20Location) false false)
  (Rendering|Components|Light|SetLightFunctionMaterial _corelight (Variables|LightSettings|GetCore%20Light%20Function))
  ;[1 1 1] Impact Light settings
  (Rendering|Components|Light|SetLightColor _impactlight (Variables|LightSettings|GetImpact%20Light%20Color) true)
  (Rendering|Components|Light|SetIntensity _impactlight (Variables|LightSettings|GetImpact%20Light%20Intensity))
  (Rendering|Lighting|SetAttenuationRadius _impactlight (Variables|LightSettings|GetImpact%20Light%20Attenuation%20Radius))
  (Rendering|Components|Light|SetCastShadows _impactlight (Variables|LightSettings|GetImpact%20Light%20Cast%20Shadows))
  (Rendering|Components|Light|SetLightFunctionMaterial _impactlight (Variables|LightSettings|GetImpact%20Light%20Function))
  ;[1 1 1] Beam Settings
  (Effects|Components|ParticleSystem|SetColorParameter _vfx_beamtest "SparkColor" (Variables|EffectColorSettings|GetEffect%20Color))
  (Effects|Components|ParticleSystem|SetFloatParameter _vfx_beamtest "SparkColorScale" (Variables|EffectColorSettings|GetBeam%20Color%20Intensity))
  (Effects|Components|ParticleSystem|SetFloatParameter _vfx_beamtest "SparkAlphaScale" (Variables|EffectColorSettings|GetBeam%20Alpha%20Intensity)))

(fn ShootArc
  (CallFunction|CEShootArc)
  (CallFunction|CEShootArc2)
  (CallFunction|CEShootArc3))