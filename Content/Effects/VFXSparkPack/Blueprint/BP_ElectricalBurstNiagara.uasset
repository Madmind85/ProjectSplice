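; Electrical burst VFX actor that pairs a Niagara spark and smoke effect with two lights and sound cues.
; The construction script applies exposed color, scale, delay and light settings to the Niagara system and both lights.
; BeginPlay starts the effect, pre-explosion light and spark sound, then loops: wait LoopDelay, play the burst sound and set the explosion light for one second.
; The shared LoopDelay also feeds Niagara for matching timing.
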(event Custom|LoopMe
  ;[1 1 1] Pre explosion time zaps
  (Utilities|FlowControl|Delay (Variables|ExplosionNiagaraSettings|GetLoop%20Delay))
  ;[1 1 1] Explosion light and sound
  (Rendering|SetVisibility (Variables|Default|GetElecExpLight) (Variables|Default|GetExplosionight) false)
  (Audio|Components|Audio|Play (Variables|Default|GetReflections_Spark_Cue) 0.0)
  (Utilities|FlowControl|Delay 1.0)
  (Rendering|SetVisibility (Variables|Default|GetElecExpLight) (Variables|Default|GetLightOff) false)
  (CallFunction|LoopMe))

(event EventBeginPlay
  ;[1 1 1] Pre explosion time zaps
  (Components|Activation|Activate (Variables|Default|GetNS_ElectricalBurstLerp) false)
  (Rendering|SetVisibility (Variables|Default|GetElectPreExpLight) (Variables|Default|GetLightOn) false)
  (Audio|Components|Audio|Play (Variables|Default|GetFire_Sparks01_Cue) 0.0)
  (Utilities|FlowControl|Delay (Variables|ExplosionNiagaraSettings|GetLoop%20Delay))
  ;[1 1 1] Explosion light and sound
  (Rendering|SetVisibility (Variables|Default|GetElecExpLight) (Variables|Default|GetExplosionight) false)
  (Audio|Components|Audio|Play (Variables|Default|GetReflections_Spark_Cue) 0.0)
  (Utilities|FlowControl|Delay 1.0)
  (Rendering|SetVisibility (Variables|Default|GetElecExpLight) (Variables|Default|GetLightOff) false)
  (CallFunction|LoopMe))

(fn ConstructionScript
  (bind _elecexplight (Variables|Default|GetElecExpLight))
  (bind _electpreexplight (Variables|Default|GetElectPreExpLight))
  (bind _ns_electricalburstlerp (Variables|Default|GetNS_ElectricalBurstLerp))
  ;[1 1 1] Pre Explosion Light Settings
  (Rendering|Components|Light|SetLightColor _electpreexplight (Variables|Pre-LightSettings|GetPre%20Light%20Color) true)
  (Rendering|Components|Light|SetIntensity _electpreexplight (Variables|Pre-LightSettings|GetPre%20Light%20Intensity))
  (Rendering|Lighting|SetAttenuationRadius _electpreexplight (Variables|Pre-LightSettings|GetPre%20Light%20Attenuation%20Radius))
  (Rendering|Components|Light|SetCastShadows _electpreexplight (Variables|GlobalLightSettings|GetCast%20Shadows))
  (Transformation|AddRelativeLocation _electpreexplight (Variables|Pre-LightSettings|GetPre%20Light%20Source) false false)
  (Rendering|Components|Light|SetLightFunctionMaterial _electpreexplight (Variables|Pre-LightSettings|GetPre%20Light%20Function%20Material))
  ;[1 1 1] Explosion Light Settings
  (Rendering|Components|Light|SetLightColor _elecexplight (Variables|ExplosionLightSettings|GetExp%20Light%20color) true)
  (Rendering|Components|Light|SetIntensity _elecexplight (Variables|ExplosionLightSettings|GetLight%20Intensity))
  (Rendering|Lighting|SetAttenuationRadius _elecexplight (Variables|ExplosionLightSettings|GetAttenuation%20Radius))
  (Rendering|Components|Light|SetCastShadows _elecexplight (Variables|GlobalLightSettings|GetCast%20Shadows))
  (Transformation|AddRelativeLocation _elecexplight (Variables|ExplosionLightSettings|GetPoint%20Light%20Loc) false false)
  (Rendering|Components|Light|SetLightFunctionMaterial _elecexplight (Variables|ExplosionLightSettings|GetExplosion%20Light%20Function%20Material))
  ;[1 1 1] Explosion Niagara Settings
  (Effects|Components|ParticleSystem|SetColorParameter _ns_electricalburstlerp "SmokeColor" (Variables|ExplosionNiagaraSettings|GetSmoke%20Color))
  (Effects|Components|ParticleSystem|SetColorParameter _ns_electricalburstlerp "SparkBurstEndColor" (Variables|ExplosionNiagaraSettings|GetSpark%20Burst%20End%20Color))
  (Effects|Components|ParticleSystem|SetFloatParameter _ns_electricalburstlerp "SparkBurstLerpOffset" (Variables|ExplosionNiagaraSettings|GetSpark%20Burst%20Lerp%20Offset))
  (Effects|Components|ParticleSystem|SetFloatParameter _ns_electricalburstlerp "SparkBurstAlphaScale" (Variables|ExplosionNiagaraSettings|GetSpark%20Loop%20AlphaScale))
  (Effects|Components|ParticleSystem|SetFloatParameter _ns_electricalburstlerp "SparkBurstColorScale" (Variables|ExplosionNiagaraSettings|GetSpark%20Burst%20Color%20Scale))
  (Effects|Components|ParticleSystem|SetColorParameter _ns_electricalburstlerp "SparkBurstColor" (Variables|ExplosionNiagaraSettings|GetSpark%20Burst%20Color))
  (Effects|Components|ParticleSystem|SetFloatParameter _ns_electricalburstlerp "SparkLoopAlphaScale" (Variables|ExplosionNiagaraSettings|GetSpark%20Loop%20AlphaScale))
  (Effects|Components|ParticleSystem|SetColorParameter _ns_electricalburstlerp "SparkLoopColor" (Variables|ExplosionNiagaraSettings|GetSpark%20Loop%20Color))
  (Effects|Components|ParticleSystem|SetFloatParameter _ns_electricalburstlerp "SparkLoopColorScale" (Variables|ExplosionNiagaraSettings|GetSpark%20Loop%20Color%20Scale))
  (Effects|Components|ParticleSystem|SetFloatParameter _ns_electricalburstlerp "LoopDelay" (Variables|ExplosionNiagaraSettings|GetLoop%20Delay))
  (Variables|ExplosionNiagaraSettings|SetLoop%20Delay (Variables|ExplosionNiagaraSettings|GetLoop%20Delay)))